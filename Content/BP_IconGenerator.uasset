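; BP_IconGenerator is a capture rig that renders a chosen static mesh in isolation, apparently for generating icons.
; SetAssetData resolves asset data to a static mesh, applies it and its first material to the Cube component, then forces a capture.
; OnMouseMove orbits the spring arm with clamped pitch and recaptures.
; The construction script restricts the SceneCaptureComponent2D to show only the Cube component.
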(event `self.OnMouseMove`
  (params (Delta :type "Vector2D Structure") (Sensitivity :type "Float (single-precision)"))
  (bind (_x _y) (`KismetMathLibrary.BreakVector2D` Delta))
  (bind (_relativerotation_roll _relativerotation_pitch _relativerotation_yaw) (`KismetMathLibrary.BreakRotator` (`SceneComponent.RelativeRotation` (`self.SpringArmComponent`))))
  (`SceneComponent.K2_SetRelativeRotation` (`self.SpringArmComponent`) (`KismetMathLibrary.MakeRotator` 0.0 (`KismetMathLibrary.FClamp` (+ _relativerotation_pitch _y) -89.0 89.0) (+ _x _relativerotation_yaw)) false false)
  (`self.ForceCapture`))

(event `self.SetAssetData`
  (params (AssetData :type "AssetData Structure (by ref)"))
  (bind _asstatic_mesh (cast `StaticMesh` (`AssetRegistryHelpers.GetAsset` AssetData)))
  (`StaticMeshComponent.SetStaticMesh` (`self.Cube`) _asstatic_mesh)
  (`PrimitiveComponent.SetMaterial` (`self.Cube`) 0 (`StaticMesh.GetMaterial` _asstatic_mesh 0))
  (`self.ForceCapture`))

(fn `UserConstructionScript`
  (`SceneCaptureComponent.ShowOnlyComponent` (`self.SceneCaptureComponent2D`) (`self.Cube`)))